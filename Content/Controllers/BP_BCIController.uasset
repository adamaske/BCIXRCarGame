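; BP_BCIController is a controller that takes brain-computer interface input over OSC and keyboard input for driving a car.
; On BeginPlay it starts a local OSC server, then logs each bundled message's address and float value and forwards them to RecieveBCIInput.
; The float is read at the message's loop index.
; Separately, Tick polls WASD to steer the car and accelerate or decelerate both car and road manager.
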(event `self.ReceiveBeginPlay`
  (bind _newparam (`self.CreateServer` "127.0.0.1" 5700))
  (add `OSCServer.OnOscBundleReceived` _newparam (delegate `OSCBundleRecieved`))
  (`self.StartServer` _newparam))

(event `OSCBundleRecieved`
  (params (Bundle :type "OSCBundle Structure (by ref)") (IPAddress :type String) (Port :type Integer))
  (bind _returnvalue (`OSCManager.GetMessagesFromBundle` Bundle))
  (for (_array_element _array_index) _returnvalue
    (bind _returnvalue_2 (`OSCManager.GetOSCMessageAddress` _array_element))
    (bind _returnvalue_3 (`OSCManager.GetOSCAddressFullPath` _returnvalue_2))
    (bind _value (`OSCManager.GetFloat` _array_element _array_index))
    (`self.RecievedInput` _returnvalue_3 _value)))

(event `self.ReceiveTick`
  (params (DeltaSeconds :type "Float (single-precision)"))
  (if (`self.IsInputKeyDown` "A")
    (bind _returnvalue (`self.GetCar`))
    (`Car.MoveRight` _returnvalue 1.0))
  (if (`self.IsInputKeyDown` "D")
    (bind _returnvalue_2 (`self.GetCar`))
    (`Car.MoveRight` _returnvalue_2 -1.0))
  (if (`self.IsInputKeyDown` "W")
    (bind _returnvalue_3 (`self.GetRoadManager`))
    (`RoadManager.Accelerate` _returnvalue_3 1.0)
    (bind _returnvalue_4 (`self.GetCar`))
    (`Car.Accelerate` _returnvalue_4 1.0)
    (elif (`self.IsInputKeyDown` "S")
      (bind _returnvalue_5 (`self.GetRoadManager`))
      (`RoadManager.Accelerate` _returnvalue_5 -1.0)
      (bind _returnvalue_6 (`self.GetCar`))
      (`Car.Deccelerate` _returnvalue_6 1.0))))

(fn `CreateServer`
  (params (IP :type String) (PORT :type Integer))
  (returns (NewParam :type "OSCServer Object Reference"))
  (bind _returnvalue (`OSCManager.CreateOSCServer` IP PORT false false "BCIServer" null))
  (bind _output_get (set `self.mServer` _returnvalue))
  (return _output_get))

(fn `RecievedInput`
  (params (Command :type String) (Value :type "Float (double-precision)"))
  (`KismetSystemLibrary.PrintString` (`KismetStringLibrary.Concat_StrStr` "Recieved " Command " with " (`KismetStringLibrary.Conv_DoubleToString` Value)))
  (`self.RecieveBCIInput` Command Value))

(fn `StartServer`
  (params (NewParam :type "OSCServer Object Reference"))
  (`OSCServer.Listen` NewParam))

(fn `StopServer`
  (`OSCServer.Stop` (`self.mServer`)))

(fn `UserConstructionScript`)